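; Robiko is the player's companion dog character, with toggleable spotlights, a sit command and timed, barked dialogue lines shown in a widget.
; Tick scales walk speed by player distance and, while it has batteries and isn't sitting, uses AIMoveTo to follow or wander.
; Interacting transfers the player's batteries to Robiko.
; A timer-based boredom switch to wandering exists, but its trigger call is unwired; straying too far resumes following.
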(event `self.ReceiveBeginPlay`
  (bind _asbp_first_person_character (cast `/Game/FirstPerson/Blueprints/BP_FirstPersonCharacter` (`GameplayStatics.GetPlayerCharacter` 0)))
  (set `self.BPPlayerRef` _asbp_first_person_character))

(event `self.ReceiveTick`
  (params (DeltaSeconds :type "Float (single-precision)"))
  (bind _bpplayerref (`self.BPPlayerRef`))
  ;[0.5 0.5 0.5] Event Tick
  (`|ExecutionSequence`
    (:`then_0`
      (`self.UpdateDistanceToPlayer`)
      (if (`self.FollowingPlayer`)
        (`self.UpdateRobikoSpeed` true)
        (else
          (`self.UpdateRobikoSpeed` false 0.25) ; if Robiko is not following the player (bored)
        )))
    (:`then_1`
      (if (== (`self.NumOfBatteries`) 0)
        _
        (elif (not (`self.Sit`))
          (if (`self.FollowingPlayer`)
            (`self.FollowsPlayer`)
            (bind _can_be_bored__ (`self.CanBeBored`))
            (if (not _can_be_bored__)
              (set `self.startToBeBored` false))
            (else
              (`self.FollowRandomPoint`)
              (bind _tofarfromplayer (`self.CanBeToFarFromPlayer`))
              (if _tofarfromplayer
                (set `self.FollowingPlayer` true)))))))
    (:`then_2`
      (if (and (`/Game/FirstPerson/Blueprints/BP_FirstPersonCharacter.IsInteracting` _bpplayerref) (== (`/Game/FirstPerson/Blueprints/BP_FirstPersonCharacter.Hit Item` _bpplayerref) self))
        (if (not (`self.HasInteracted`))
          (set `self.HasInteracted` true)
          (set `self.NumOfBatteries` (+ (`/Game/FirstPerson/Blueprints/BP_FirstPersonCharacter.NumOfBatteries` (`self.BPPlayerRef`)) (`self.NumOfBatteries`)))
          (set `/Game/FirstPerson/Blueprints/BP_FirstPersonCharacter.NumOfBatteries` 0 (`self.BPPlayerRef`))
          (`KismetSystemLibrary.Delay` 1.0)
          (set `self.HasInteracted` false))))))

(event `UpdateDistanceToPlayer`
  ;[0 0 0] Update the distance to the player
  (set `self.DistanceToPlayer` (`self.GetDistanceTo` self (`GameplayStatics.GetPlayerCharacter` 0))))

(event `UpdateRobikoSpeed`
  (params (speedByDistanceToPlayer :type Boolean) (speedMultiplayer :type "Float (double-precision)"))
  ;[0 0 0] Update Robiko Speed
  (if speedByDistanceToPlayer
    (set `CharacterMovementComponent.MaxWalkSpeed` (* (`self.MaxSpeed`) (/ (`self.DistanceToPlayer`) (- (`self.ToFarFromPlayer`) (`self.ToNearFromPlayer`)))) (`self.CharacterMovement`)) ; Set the speed according to the distance with the player
    (else
      (set `CharacterMovementComponent.MaxWalkSpeed` (* (`self.MaxSpeed`) speedMultiplayer) (`self.CharacterMovement`)) ; Set the speed according to the float sended
    )))

(event `StartsToBeBored`
  ;[0.0838 0.349 0.09819] Robiko is bored
  (if (not (`self.startToBeBored`))
    (set `self.startToBeBored` true)
    (`KismetSystemLibrary.K2_SetTimerDelegate` (delegate `RobikoIsBored`) (`self.TimeToGetBored`))))

(event `RobikoIsBored`
  ;[0.0838 0.349 0.09819] Robiko is bored
  (bind _can_be_bored__ (`self.CanBeBored`))
  (if _can_be_bored__
    (set `self.startToBeBored` false)
    (set `self.FollowingPlayer` false)))

(event `FollowRandomPoint`
  ;[0.06274 0.2745 0.2588] Set a random point to move if Robiko it's not folllowing the player and it's a certain distance of the player
  (`KismetSystemLibrary.Delay` (`KismetMathLibrary.RandomFloatInRange` 1.0 3.0))
  (`|AIMoveTo` self (`NavigationSystemV1.K2_GetRandomReachablePointInRadius` (`self.K2_GetActorLocation`) (/ (`self.ToFarFromPlayer`) 2.0) null null) null))

(event `FollowsPlayer`
  ;[0.06274 0.2745 0.2588] Follows the player
  (bind _asbp_first_person_character (cast `/Game/FirstPerson/Blueprints/BP_FirstPersonCharacter` (`GameplayStatics.GetPlayerCharacter` 0)))
  (`|AIMoveTo` self (0.0 0.0 0.0) _asbp_first_person_character (`self.ToNearFromPlayer`)))

(event `ChangeFlashlight`
  ;[0.1568 0.1771 0.04279] Flashlight activate and desactivate
  (`SceneComponent.SetVisibility` (`self.SpotLight1`) (not (`SceneComponent.bVisible` (`self.SpotLight1`))) false)
  (`SceneComponent.SetVisibility` (`self.SpotLight2`) (not (`SceneComponent.bVisible` (`self.SpotLight2`))) false)
  (`GameplayStatics.PlaySoundAtLocation` "/Game/_Master/AudioSource/lantern_off_2.lantern_off_2" (`self.K2_GetActorLocation`) (struct) 1.0 1.0 0.0 null null null null))

(event `SitByPlayer`
  (params (PositionToSit :type "Vector Structure"))
  (bind _billboard (`self.Billboard`))
  ;[0.7893 0.3989 1] Sit the dog by activating and desactivating the charater movement
  (`/Engine/EditorBlueprintResources/StandardMacros.FlipFlop`
    (:`A`
      (`SceneComponent.K2_SetWorldLocation` _billboard PositionToSit false false)
      (`SceneComponent.SetVisibility` _billboard true false)
      (set `self.Sit` true)
      (`|AIMoveTo` self PositionToSit null 1.0
        (:`OnSuccess`
          (`ActorComponent.Deactivate` (`self.CharacterMovement`))
          (`SceneComponent.SetVisibility` (`self.Billboard`) false false))))
    (:`B`
      (set `self.Sit` false)
      (`ActorComponent.SetActive` (`self.CharacterMovement`) true false))))

(event `/Game/_Master/Robiko/Blueprints/BPI_Dialogue.Talk`
  ;[0.5312 0.411 0.2002] Talk message, appears the UI dialogue and desapears and also delete the last dialogue
  (`/Engine/EditorBlueprintResources/StandardMacros.IncrementInt` (`self.TalkIndex`)
    (:`  `
      (if (< (`self.TalkIndex`) (`KismetArrayLibrary.Array_Length` (`self.Dialogue`)))
        (`self.UITalkDialogue`
          (:`then`
            _)
          (:`else`
            (bind _returnvalue (`|CreateWidget` "/Game/FirstPerson/UI/WD_dialogue.WD_dialogue_C" (`GameplayStatics.GetPlayerController` 0)))
            (bind _output_get (set `self.UITalkDialogue` _returnvalue))
            (`UserWidget.AddToViewport` _output_get 0)))
        (`TextBlock.SetText` (`/Game/FirstPerson/UI/WD_dialogue.TalkText` (`self.UITalkDialogue`)) (`KismetTextLibrary.Conv_StringToText` (`|GetArrayItem` (`self.Dialogue`) (`self.TalkIndex`))))
        (`GameplayStatics.PlaySoundAtLocation` "/Game/_Master/Robiko/Audio/robiko_bark_3.robiko_bark_3" (`self.K2_GetActorLocation`) (struct) 1.0 1.0 0.0 null null null null)
        (`KismetSystemLibrary.Delay` 4.0)
        (`/Game/_Master/Robiko/Blueprints/BPI_Dialogue.Talk`)
        (else
          (`Widget.RemoveFromParent` (`self.UITalkDialogue`))
          (`SceneComponent.SetVisibility` (`self.InnerInteractIcon`) false false)
          (`KismetArrayLibrary.Array_Clear` (`self.Dialogue`)))))))

(event `self.Sphere.OnComponentBeginOverlap`
  (params (OverlappedComponent :type "PrimitiveComponent Object Reference") (OtherActor :type "Actor Object Reference") (OtherComp :type "PrimitiveComponent Object Reference") (OtherBodyIndex :type Integer) (bFromSweep :type Boolean) (SweepResult :type "HitResult Structure (by ref)"))
  ;[0 0 0] icon interact appeareance logic
  (if (and (== OtherActor (`GameplayStatics.GetPlayerCharacter` 0)) (< (`self.TalkIndex`) (`KismetArrayLibrary.Array_Length` (`self.Dialogue`))))
    (`SceneComponent.SetVisibility` (`self.InnerInteractIcon`) true false)))

(event `self.Sphere.OnComponentEndOverlap`
  (params (OverlappedComponent :type "PrimitiveComponent Object Reference") (OtherActor :type "Actor Object Reference") (OtherComp :type "PrimitiveComponent Object Reference") (OtherBodyIndex :type Integer))
  ;[0 0 0] icon interact appeareance logic
  (if (== OtherActor (`GameplayStatics.GetPlayerCharacter` 0))
    (`SceneComponent.SetVisibility` (`self.InnerInteractIcon`) false false)))

(fn `CanBeBored`
  (returns (`can be bored ?` :type Boolean))
  (return (and (<= (`self.DistanceToPlayer`) (+ (`self.ToNearFromPlayer`) 100.0)) (<= (`KismetArrayLibrary.Array_Length` (`self.Dialogue`)) 0) (not (`self.Sit`)))))

(fn `CanBeToFarFromPlayer`
  (returns (ToFarFromPlayer :type Boolean))
  (return (not (`KismetMathLibrary.InRange_FloatFloat` (`self.DistanceToPlayer`) 0.0 (/ (`self.ToFarFromPlayer`) 2.0)))))

(fn `Interact`
  (params (Interactor :type "Character Object Reference"))
  (returns (`DidInteract?` :type Boolean))
  (return false))

(fn `UserConstructionScript`)