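; Elevator actor with a sliding door, controllable rect light and animated Back surface, driven through custom events.
; A dynamic material on Back gets a base Speed at BeginPlay, which StartDecrease offsets through the SpeedIncrease timeline.
; Light events switch it on, off or to a flickering light function.
; Door events slide LiftDoor along X with a computed duration; opening also hides Back and disables its collision.
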(event `self.ReceiveBeginPlay`
  (bind _returnvalue (`PrimitiveComponent.CreateDynamicMaterialInstance` (`self.back`) 0 null "None"))
  (`MaterialInstanceDynamic.SetVectorParameterValue` _returnvalue "Speed" (`KismetMathLibrary.MakeColor` 0.0 (`self.G`))))

(event `FlickerinLight`
  (`LightComponent.SetLightFunctionMaterial` (`self.RectLight`) "/Game/_Master/Materials/M_flikering_light.M_flikering_light"))

(event `StartDecrease`
  (bind (_direction _speed) (`Timeline|SpeedIncrease` :!via `PlayFromStart`)
    (:`Update`
      (`MaterialInstanceDynamic.SetVectorParameterValue` (stale `self.ReceiveBeginPlay` _returnvalue) "Speed" (`KismetMathLibrary.MakeColor` 0.0 (+ _speed (`self.G`)))))))

(event `PutOffLight`
  (`LightComponent.SetIntensity` (`self.RectLight`) 0.0))

(event `PutOnLight`
  (`LightComponent.SetIntensity` (`self.RectLight`) 200.0))

(event `CloseDoor`
  ;[0.2188 0.05793 0.1135] Event to move door
  (`self.HandleMovementDoor` -110.0))

(event `OpenDoor`
  (bind _back (`self.back`))
  ;[0.2188 0.05793 0.1135] Event to move door
  (`self.HandleMovementDoor` -310.0)
  (`SceneComponent.SetVisibility` _back false false)
  (`PrimitiveComponent.SetCollisionEnabled` _back "NoCollision"))

(event `HandleMovementDoor`
  (params (SetPositionX :type "Float (double-precision)"))
  (bind _liftdoor (`self.LiftDoor`))
  (bind (_relativelocation_x _relativelocation_y _relativelocation_z) (`KismetMathLibrary.BreakVector` (`SceneComponent.RelativeLocation` _liftdoor)))
  ;[0.1302 0.1302 0.1302] Handle Movement Door
  (`KismetSystemLibrary.MoveComponentTo` _liftdoor (`KismetMathLibrary.MakeVector` SetPositionX _relativelocation_y _relativelocation_z) (struct) false false (/ (`KismetMathLibrary.Vector_Distance` (`KismetMathLibrary.MakeVector` _relativelocation_x _relativelocation_y _relativelocation_z) (`KismetMathLibrary.MakeVector` _relativelocation_x SetPositionX _relativelocation_z)) 100.0)))

(fn `UserConstructionScript`)