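; BP_Item is an interactable item actor that shows proximity icons to the player and provides an Interact function that only returns false.
; Inner and outer sphere collisions, sized from radius variables in the construction script, toggle two icons as the player overlaps.
; The outer icon appears at range and swaps to the inner icon up close.
; BeginPlay caches the BP_FirstPersonCharacter player reference.
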(event `self.ReceiveBeginPlay`
  (bind _asbp_first_person_character (cast `/Game/FirstPerson/Blueprints/BP_FirstPersonCharacter` (`GameplayStatics.GetPlayerCharacter` 0)))
  (set `self.BPPlayerRef` _asbp_first_person_character))

(event `self.InnerSphereCollision.OnComponentBeginOverlap`
  (params (OverlappedComponent :type "PrimitiveComponent Object Reference") (OtherActor :type "Actor Object Reference") (OtherComp :type "PrimitiveComponent Object Reference") (OtherBodyIndex :type Integer) (bFromSweep :type Boolean) (SweepResult :type "HitResult Structure (by ref)"))
  ;[0.2135 0.0823 0.0823] Interaction icon appearance
  (if (== OtherActor (`GameplayStatics.GetPlayerCharacter` 0))
    (`SceneComponent.SetVisibility` (`self.InnerInteractIcon`) true false)
    (`SceneComponent.SetVisibility` (`self.OuterInteractIcon`) false false)))

(event `self.InnerSphereCollision.OnComponentEndOverlap`
  (params (OverlappedComponent :type "PrimitiveComponent Object Reference") (OtherActor :type "Actor Object Reference") (OtherComp :type "PrimitiveComponent Object Reference") (OtherBodyIndex :type Integer))
  ;[0.2135 0.0823 0.0823] Interaction icon appearance
  (if (== (`GameplayStatics.GetPlayerCharacter` 0) OtherActor)
    (`SceneComponent.SetVisibility` (`self.InnerInteractIcon`) false false)
    (`SceneComponent.SetVisibility` (`self.OuterInteractIcon`) true false)))

(event `self.OuterSphereCollision.OnComponentBeginOverlap`
  (params (OverlappedComponent :type "PrimitiveComponent Object Reference") (OtherActor :type "Actor Object Reference") (OtherComp :type "PrimitiveComponent Object Reference") (OtherBodyIndex :type Integer) (bFromSweep :type Boolean) (SweepResult :type "HitResult Structure (by ref)"))
  ;[0.2135 0.0823 0.0823] Interaction icon appearance
  (if (== OtherActor (`GameplayStatics.GetPlayerCharacter` 0))
    (`SceneComponent.SetVisibility` (`self.OuterInteractIcon`) true false)))

(event `self.OuterSphereCollision.OnComponentEndOverlap`
  (params (OverlappedComponent :type "PrimitiveComponent Object Reference") (OtherActor :type "Actor Object Reference") (OtherComp :type "PrimitiveComponent Object Reference") (OtherBodyIndex :type Integer))
  ;[0.2135 0.0823 0.0823] Interaction icon appearance
  (if (== (`GameplayStatics.GetPlayerCharacter` 0) OtherActor)
    (`SceneComponent.SetVisibility` (`self.OuterInteractIcon`) false false)))

(fn `Interact`
  (params (Interactor :type "Character Object Reference"))
  (returns (`DidInteract?` :type Boolean))
  (return false))

(fn `UserConstructionScript`
  (`SphereComponent.SetSphereRadius` (`self.OuterSphereCollision`) (`self.OuterRadiusCollision`) true)
  (`SphereComponent.SetSphereRadius` (`self.InnerSphereCollision`) (`self.InnerRadiusCollision`) true))