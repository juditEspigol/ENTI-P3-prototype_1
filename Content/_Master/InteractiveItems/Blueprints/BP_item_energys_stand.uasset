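; Interactive battery stand item that the player can pick up once for energy.
; Each tick it checks whether the player is interacting with it as the hit item and, if not yet picked, triggers the pickup.
; Pickup destroys the battery mesh, plays a sound, credits the player through its PickUpBattery call, swaps the frame material and hides both interact icons.
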(event `self.ReceiveTick`
  (params (DeltaSeconds :type "Float (single-precision)"))
  (bind _bpplayerref (`self.BPPlayerRef`))
  (`parent.ReceiveTick` 0.0)
  (if (and (`/Game/FirstPerson/Blueprints/BP_FirstPersonCharacter.IsInteracting` _bpplayerref) (== (`/Game/FirstPerson/Blueprints/BP_FirstPersonCharacter.Hit Item` _bpplayerref) self))
    (if (not (`self.HasBeenPicked`))
      (`self.PickUpBattery`))))

(event `PickUpBattery`
  ;[0.3281 0.3248 0.05379] Picked Up Battery Interaction (1 frame)
  (`ActorComponent.K2_DestroyComponent` (`self.Battery_StaticMesh`))
  (`GameplayStatics.PlaySoundAtLocation` "/Game/_Master/AudioSource/PickUp_Battery_1.PickUp_Battery_1" (`self.K2_GetActorLocation`) (struct) 1.5 1.0 0.0 null null null null)
  (`/Game/FirstPerson/Blueprints/BP_FirstPersonCharacter.PickUpBattery` (`self.BPPlayerRef`) 2)
  (set `self.HasBeenPicked` true)
  (`PrimitiveComponent.SetMaterial` (`self.Frame_StaticMesh`) 0 "/Game/StarterContent/Materials/M_Tech_Hex_Tile.M_Tech_Hex_Tile")
  (`SceneComponent.SetVisibility` (`self.OuterInteractIcon`) false false)
  (`SceneComponent.SetVisibility` (`self.InnerInteractIcon`) false false))

(fn `UserConstructionScript`
  (`parent.UserConstructionScript`))