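; BP_Item_Battery is an interactive battery pickup that the player collects by interacting with it.
; It polls on Tick for the player interacting with this actor as the hit item, guarded to fire once.
; Pickup passes the battery price to the player, plays a sound, and destroys the actor after a short delay.
; If the motor reference is valid, it then sends pickup messages to the motor and battery box.
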(event `self.ReceiveTick`
  (params (DeltaSeconds :type "Float (single-precision)"))
  (bind _bpplayerref (`self.BPPlayerRef`))
  (`parent.ReceiveTick` 0.0)
  (if (and (`/Game/FirstPerson/Blueprints/BP_FirstPersonCharacter.IsInteracting` _bpplayerref) (== (`/Game/FirstPerson/Blueprints/BP_FirstPersonCharacter.Hit Item` _bpplayerref) self))
    (if (not (`self.HasBeenPicked`))
      (`self.PickUpBattery`))))

(event `PickUpBattery`
  (bind _bpmotorref (`self.BPMotorRef`))
  ;[0.3281 0.3248 0.05379] Picked Up Battery Interaction (1 frame)
  (set `self.HasBeenPicked` true)
  (`/Game/FirstPerson/Blueprints/BP_FirstPersonCharacter.PickUpBattery` (`self.BPPlayerRef`) (`self.BatteryPrice`))
  (`GameplayStatics.PlaySoundAtLocation` "/Game/_Master/AudioSource/SW_pickup_battery_1.SW_pickup_battery_1" (`self.K2_GetActorLocation`) (struct) 1.5 1.0 0.0 null null null null)
  (`KismetSystemLibrary.Delay` 0.1)
  (`self.K2_DestroyActor`)
  (if (`KismetSystemLibrary.IsValid` _bpmotorref)
    (message `/Game/_Master/InteractiveItems/Blueprints/BPI_door.PickUpKey` _bpmotorref)
    (message `/Game/_Master/InteractiveItems/Blueprints/BPI_door.PickUpKey` (`self.BRBatteryBox`))))

(fn `UserConstructionScript`
  (`parent.UserConstructionScript`))