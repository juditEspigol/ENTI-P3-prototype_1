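; Key-locked interactive door that cycles through partially open, fully open and closed, swinging by the player's facing direction.
; Tick polls the player's IsInteracting and HitItem, interpolating yaw with FInterpTo while a timer advances the state, and playing a sound per move.
; Without a key it plays a locked sound; PickUpKey unlocks it.
; Two overlap spheres, sized in the construction script, toggle far and near interaction icons, the near one showing lock status.
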(event `self.ReceiveBeginPlay`
  (bind _asbp_first_person_character (cast `/Game/FirstPerson/Blueprints/BP_FirstPersonCharacter` (`GameplayStatics.GetPlayerCharacter` 0)))
  (set `self.BPPlayerRef` _asbp_first_person_character))

(event `self.ReceiveTick`
  (params (DeltaSeconds :type "Float (single-precision)"))
  (bind _bpplayerref (`self.BPPlayerRef`))
  (if (and (`/Game/FirstPerson/Blueprints/BP_FirstPersonCharacter.IsInteracting` _bpplayerref) (== (`/Game/FirstPerson/Blueprints/BP_FirstPersonCharacter.Hit Item` _bpplayerref) self))
    (if (`self.HasKey`)
      (if (`self.bIsInteractingWithDoor`)
        (`self.HandleDoor`) ; More than 1 frame
        (else
          (`self.IsInteractingWithDoor` (`self.BPPlayerRef`))
          (bind _foundwidgets (`WidgetBlueprintLibrary.GetAllWidgetsOfClass` "/Game/FirstPerson/UI/WD_PickUpKey.WD_PickUpKey_C"))
          (`Widget.RemoveFromParent` _foundwidgets)))
      (else
        (`self.CanNOTOpenDoor`)))))

(event `IsInteractingWithDoor`
  (params (Player :type "/Game/FirstPerson/Blueprints/BP_FirstPersonCharacter Object Reference"))
  ;[0.3438 0.213 0] Door Interaction Mathematics
  (if (> (`KismetMathLibrary.Dot_VectorVector` (`self.GetActorForwardVector` Player) (`SceneComponent.GetForwardVector` (`self.DoorOpeningLocation`))) 0.0)
    (set `self.DoorOpenSide` 1.0)
    (else
      (set `self.DoorOpenSide` -1.0)))
  (set `self.bIsInteractingWithDoor` true)
  (`KismetSystemLibrary.K2_SetTimerDelegate` (delegate `StopInteractingWithDoor`) (`self.DoorSoundTime`)))

(event `StopInteractingWithDoor`
  ;[0.3438 0.213 0] Door Interaction Mathematics
  (set `self.bIsInteractingWithDoor` false)
  (switch `/Game/_Master/InteractiveItems/Blueprints/E_DoorStates` (`self.EDoorStates`)
    (:`NewEnumerator2`
      (set `self.EDoorStates` "NewEnumerator0"))
    (:`NewEnumerator0`
      (set `self.EDoorStates` "NewEnumerator1"))
    (:`NewEnumerator1`
      (set `self.EDoorStates` "NewEnumerator2")))
  (set `self.PlaySound` true))

(event `HandleDoor`
  ;[0.01229 0.05286 0.0356] Handle Door (Rotating Door acoording to our current door state)
  (switch `/Game/_Master/InteractiveItems/Blueprints/E_DoorStates` (`self.EDoorStates`)
    (:`NewEnumerator2`
      (`self.HandleRotation` (* 20.0 (`self.DoorOpenSide`)))
      (if (`self.PlaySound`)
        (`GameplayStatics.PlaySoundAtLocation` "/Game/_Master/AudioSource/door_partially_open.door_partially_open" (`self.K2_GetActorLocation`) (struct) 3.0 1.0 0.0 null null null null)
        (set `self.PlaySound` false)))
    (:`NewEnumerator0`
      (`self.HandleRotation` (* (`self.DoorOpenAngle`) (`self.DoorOpenSide`)))
      (if (`self.PlaySound`)
        (`GameplayStatics.PlaySoundAtLocation` "/Game/_Master/AudioSource/door_totally_open.door_totally_open" (`self.K2_GetActorLocation`) (struct) 2.0 1.0 0.0 null null null null)
        (set `self.PlaySound` false)))
    (:`NewEnumerator1`
      (`self.HandleRotation` 0.0)
      (if (`self.PlaySound`)
        (`GameplayStatics.PlaySoundAtLocation` "/Game/_Master/AudioSource/door_close_1.door_close_1" (`self.K2_GetActorLocation`) (struct) 1.0 1.0 0.0 null null null null)
        (set `self.PlaySound` false)))))

(event `HandleRotation`
  (params (SetRotation :type "Float (double-precision)"))
  ;[0.0295 0.1302 0.08736] Handle Rotation
  (`SceneComponent.K2_SetRelativeRotation` (`self.Door`) (`KismetMathLibrary.MakeRotator` 0.0 0.0 (`KismetMathLibrary.FInterpTo` (.yaw (`SceneComponent.RelativeRotation` (`self.Door`))) SetRotation (`GameplayStatics.GetWorldDeltaSeconds`) (`self.Interp Speed`))) false false))

(event `CanNOTOpenDoor`
  ;[0.1075 0.1354 0.1045] Play sound when player don't have key
  (if (`self.PlaySound`)
    (`GameplayStatics.PlaySoundAtLocation` "/Game/_Master/AudioSource/Need_Key_2.Need_Key_2" (`self.K2_GetActorLocation`) (struct) 1.0 1.0 0.0 null null null null)
    (set `self.PlaySound` false)
    (`KismetSystemLibrary.Delay` (`self.DoorSoundTime`))
    (set `self.PlaySound` true)))

(event `/Game/_Master/InteractiveItems/Blueprints/BPI_DoorInterface.PickUpKey`
  (set `self.HasKey` true))

(event `self.InnerSphereCollision.OnComponentBeginOverlap`
  (params (OverlappedComponent :type "PrimitiveComponent Object Reference") (OtherActor :type "Actor Object Reference") (OtherComp :type "PrimitiveComponent Object Reference") (OtherBodyIndex :type Integer) (bFromSweep :type Boolean) (SweepResult :type "HitResult Structure (by ref)"))
  ;[0.2135 0.0823 0.0823] Interaction icon appearance
  (if (== OtherActor (`GameplayStatics.GetPlayerCharacter` 0))
    (`SceneComponent.SetVisibility` (`self.InnerInteractIcon1`) true false)
    (`SceneComponent.SetVisibility` (`self.InnerInteractIcon2`) true false)
    (`SceneComponent.SetVisibility` (`self.OuterInteractIcon1`) false false)
    (`SceneComponent.SetVisibility` (`self.OuterInteractIcon2`) false false)
    (if (`self.HasKey`)
      (`BillboardComponent.SetSprite` (`self.InnerInteractIcon2`) "/Game/_Master/InteractiveItems/Textures/T_interact_icon.T_interact_icon")
      (`BillboardComponent.SetSprite` (`self.InnerInteractIcon1`) "/Game/_Master/InteractiveItems/Textures/T_interact_icon.T_interact_icon")
      (else
        (`BillboardComponent.SetSprite` (`self.InnerInteractIcon2`) "/Game/_Master/InteractiveItems/Textures/interact_Icon_closed.interact_Icon_closed")
        (`BillboardComponent.SetSprite` (`self.InnerInteractIcon1`) "/Game/_Master/InteractiveItems/Textures/interact_Icon_closed.interact_Icon_closed")))))

(event `self.InnerSphereCollision.OnComponentEndOverlap`
  (params (OverlappedComponent :type "PrimitiveComponent Object Reference") (OtherActor :type "Actor Object Reference") (OtherComp :type "PrimitiveComponent Object Reference") (OtherBodyIndex :type Integer))
  ;[0.2135 0.0823 0.0823] Interaction icon appearance
  (if (== (`GameplayStatics.GetPlayerCharacter` 0) OtherActor)
    (`SceneComponent.SetVisibility` (`self.InnerInteractIcon1`) false false)
    (`SceneComponent.SetVisibility` (`self.InnerInteractIcon2`) false false)
    (`SceneComponent.SetVisibility` (`self.OuterInteractIcon1`) true false)
    (`SceneComponent.SetVisibility` (`self.OuterInteractIcon2`) true false)))

(event `self.OuterSphereCollision.OnComponentBeginOverlap`
  (params (OverlappedComponent :type "PrimitiveComponent Object Reference") (OtherActor :type "Actor Object Reference") (OtherComp :type "PrimitiveComponent Object Reference") (OtherBodyIndex :type Integer) (bFromSweep :type Boolean) (SweepResult :type "HitResult Structure (by ref)"))
  ;[0.2135 0.0823 0.0823] Interaction icon appearance
  (if (== OtherActor (`GameplayStatics.GetPlayerCharacter` 0))
    (`SceneComponent.SetVisibility` (`self.OuterInteractIcon1`) true false)
    (`SceneComponent.SetVisibility` (`self.OuterInteractIcon2`) true false)))

(event `self.OuterSphereCollision.OnComponentEndOverlap`
  (params (OverlappedComponent :type "PrimitiveComponent Object Reference") (OtherActor :type "Actor Object Reference") (OtherComp :type "PrimitiveComponent Object Reference") (OtherBodyIndex :type Integer))
  ;[0.2135 0.0823 0.0823] Interaction icon appearance
  (if (== (`GameplayStatics.GetPlayerCharacter` 0) OtherActor)
    (`SceneComponent.SetVisibility` (`self.OuterInteractIcon1`) false false)
    (`SceneComponent.SetVisibility` (`self.OuterInteractIcon2`) false false)))

(fn `Interact`
  (params (Interactor :type "Character Object Reference"))
  (returns (`DidInteract?` :type Boolean))
  (return false))

(fn `UserConstructionScript`
  (`SphereComponent.SetSphereRadius` (`self.OuterSphereCollision`) (`self.OuterRadiusCollision`) true)
  (`SphereComponent.SetSphereRadius` (`self.InnerSphereCollision`) (`self.InnerRadiusCollision`) true))