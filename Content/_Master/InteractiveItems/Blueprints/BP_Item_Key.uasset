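; BP_Item_Key is an interactive key item that the player picks up, notifying a linked door.
; Tick polls the player reference and triggers the pickup once when the player is interacting and the key is the hit item.
; Pickup sends a message to the door, plays a sound, then after a short delay destroys the actor and shows a pickup widget.
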(event `self.ReceiveTick`
  (params (DeltaSeconds :type "Float (single-precision)"))
  (bind _bpplayerref (`self.BPPlayerRef`))
  (`parent.ReceiveTick` 0.0)
  (if (and (`/Game/FirstPerson/Blueprints/BP_FirstPersonCharacter.IsInteracting` _bpplayerref) (== (`/Game/FirstPerson/Blueprints/BP_FirstPersonCharacter.Hit Item` _bpplayerref) self))
    (if (not (`self.HasBeenPicked`))
      (`self.PickUpKey`))))

(event `PickUpKey`
  ;[0.224 0.1931 0.07535] Pick up Key Interaction
  (set `self.HasBeenPicked` true)
  (message `/Game/_Master/InteractiveItems/Blueprints/BPI_door.PickUpKey` (`self.BPDoor`))
  (`GameplayStatics.PlaySoundAtLocation` "/Game/_Master/AudioSource/SW_pickup_key_1.SW_pickup_key_1" (`self.K2_GetActorLocation`) (struct) 1.0 1.0 0.0 null null null null)
  (`KismetSystemLibrary.Delay` 0.1)
  (`self.K2_DestroyActor`)
  (bind _returnvalue (`|CreateWidget` "/Game/FirstPerson/UI/WD_pickup_key.WD_pickup_key_C" (`GameplayStatics.GetPlayerController` 0)))
  (`UserWidget.AddToViewport` _returnvalue 0))

(fn `UserConstructionScript`
  (`parent.UserConstructionScript`))