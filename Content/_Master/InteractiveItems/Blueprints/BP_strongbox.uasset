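; BP_strongbox is an interactive strongbox whose Cube door slides open and closed as characters enter and leave its Box trigger.
; Overlaps by BR_RobikoCharacter or player character 0 call OpenDoor or CloseDoor, printing debug text.
; Both feed HandleMovementDoor, which moves the Cube along relative X, slower opening than closing.
; Move duration divides distance by speed, but measures that distance between current Y and target X.
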(event `CloseDoor`
  (set `self.VelocitySpeed` 120.0)
  (`self.HandleMovementDoor` -48.0))

(event `HandleMovementDoor`
  (params (SetPositionX :type "Float (double-precision)"))
  (bind _cube (`self.Cube`))
  (bind (_relativelocation_x _relativelocation_y _relativelocation_z) (`KismetMathLibrary.BreakVector` (`SceneComponent.RelativeLocation` _cube)))
  (`KismetSystemLibrary.MoveComponentTo` _cube (`KismetMathLibrary.MakeVector` SetPositionX _relativelocation_y _relativelocation_z) (struct) false false (/ (`KismetMathLibrary.Vector_Distance` (`KismetMathLibrary.MakeVector` _relativelocation_x _relativelocation_y _relativelocation_z) (`KismetMathLibrary.MakeVector` _relativelocation_x SetPositionX _relativelocation_z)) (`self.VelocitySpeed`))))

(event `OpenDoor`
  (set `self.VelocitySpeed` 20.0)
  (`self.HandleMovementDoor` 48.0))

(event `self.Box.OnComponentBeginOverlap`
  (params (OverlappedComponent :type "PrimitiveComponent Object Reference") (OtherActor :type "Actor Object Reference") (OtherComp :type "PrimitiveComponent Object Reference") (OtherBodyIndex :type Integer) (bFromSweep :type Boolean) (SweepResult :type "HitResult Structure (by ref)"))
  (`|ExecutionSequence`
    (:`then_0`
      (cast `/Game/_Master/Robiko/Blueprints/BR_RobikoCharacter` OtherActor)
      (`self.OpenDoor` :!label _label)
      (`KismetSystemLibrary.PrintString` "enter"))
    (:`then_1`
      (if (== OtherActor (`GameplayStatics.GetPlayerCharacter` 0))
        (goto _label)))))

(event `self.Box.OnComponentEndOverlap`
  (params (OverlappedComponent :type "PrimitiveComponent Object Reference") (OtherActor :type "Actor Object Reference") (OtherComp :type "PrimitiveComponent Object Reference") (OtherBodyIndex :type Integer))
  (`|ExecutionSequence`
    (:`then_0`
      (cast `/Game/_Master/Robiko/Blueprints/BR_RobikoCharacter` OtherActor)
      (`self.CloseDoor` :!label _label_2)
      (`KismetSystemLibrary.PrintString` "exit" true true (struct :`R` 1.0 :`G` 0.069179 :`B` 0.561482 :`A` 1.0)))
    (:`then_1`
      (if (== OtherActor (`GameplayStatics.GetPlayerCharacter` 0))
        (goto _label_2)))))

(fn `UserConstructionScript`)