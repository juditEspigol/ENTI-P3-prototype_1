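; BP_elevator_motor is an interactive elevator motor that shows a battery and a pulsing frame material when powered.
; PickUpKey arms it, then Tick polls the cached first-person character and powers the visuals while the player interacts with this actor.
; Activated and Desactivated events set the same battery visibility and frame material on or off directly.
; The Interact function is a stub returning false.
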(event `self.ReceiveBeginPlay`
  (bind _asbp_first_person_character (cast `/Game/FirstPerson/Blueprints/BP_FirstPersonCharacter` (`GameplayStatics.GetPlayerCharacter` 0)))
  (set `self.BPPlayerRef` _asbp_first_person_character))

(event `self.ReceiveTick`
  (params (DeltaSeconds :type "Float (single-precision)"))
  (bind _bpplayerref (`self.BPPlayerRef`))
  (if (and (`/Game/FirstPerson/Blueprints/BP_FirstPersonCharacter.IsInteracting` _bpplayerref) (== (`/Game/FirstPerson/Blueprints/BP_FirstPersonCharacter.Hit Item` _bpplayerref) self))
    (if (`self.HasInteract`)
      (`SceneComponent.SetVisibility` (`self.Battery_StaticMesh`) true false)
      (`PrimitiveComponent.SetMaterial` (`self.Frame_StaticMesh`) 0 "/Game/StarterContent/Materials/M_Tech_Hex_Tile_Pulse.M_Tech_Hex_Tile_Pulse"))))

(event `/Game/_Master/InteractiveItems/Blueprints/BPI_door.PickUpKey`
  (set `self.HasInteract` true))

(event `Activated`
  (`SceneComponent.SetVisibility` (`self.Battery_StaticMesh`) true false)
  (`PrimitiveComponent.SetMaterial` (`self.Frame_StaticMesh`) 0 "/Game/StarterContent/Materials/M_Tech_Hex_Tile_Pulse.M_Tech_Hex_Tile_Pulse"))

(event `Desactivated`
  (`SceneComponent.SetVisibility` (`self.Battery_StaticMesh`) false false)
  (`PrimitiveComponent.SetMaterial` (`self.Frame_StaticMesh`) 0 "/Game/StarterContent/Materials/M_Tech_Hex_Tile.M_Tech_Hex_Tile"))

(fn `Interact`
  (params (Interactor :type "Character Object Reference"))
  (returns (`DidInteract?` :type Boolean))
  (return false))

(fn `UserConstructionScript`)