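; BP_Item_Note is an interactive note item that the player picks up to read in an on-screen widget.
; Tick polls the player reference for an interaction hitting this actor, with a flag preventing repeat pickups.
; Pickup hides the note, plays a page sound, shows the WB_robiko_instructions widget, blocks move and look input, and flags the player.
; DropItem removes the widget, unhides the note and restores input.
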(event `self.ReceiveTick`
  (params (DeltaSeconds :type "Float (single-precision)"))
  (bind _bpplayerref (`self.BPPlayerRef`))
  ;[0.5 0.5 0.5] Event Tick
  (if (and (`/Game/FirstPerson/Blueprints/BP_FirstPersonCharacter.IsInteracting` _bpplayerref) (== (`/Game/FirstPerson/Blueprints/BP_FirstPersonCharacter.Hit Item` _bpplayerref) self))
    (if (not (`self.HasBeenPicked`))
      (`self.PickUpItem`))))

(event `PickUpItem`
  (bind _returnvalue (`GameplayStatics.GetPlayerController` 0))
  ;[0 0 0] Pick Up Note and adding to the viewport
  (set `self.HasBeenPicked` true)
  (`self.SetActorHiddenInGame` true)
  (`GameplayStatics.PlaySoundAtLocation` "/Game/_Master/AudioSource/PickUp_Page_1.PickUp_Page_1" (`self.K2_GetActorLocation`) (struct) 1.0 1.0 0.0 null null null null)
  (bind _returnvalue_2 (`|CreateWidget` "/Game/_Master/InteractiveItems/UI/WB_robiko_instructions.WB_robiko_instructions_C"))
  (bind _output_get (set `self.WB Note Ref` _returnvalue_2))
  (`UserWidget.AddToViewport` _output_get 0)
  (`Controller.SetIgnoreMoveInput` _returnvalue true)
  (`Controller.SetIgnoreLookInput` _returnvalue true)
  (set `/Game/FirstPerson/Blueprints/BP_FirstPersonCharacter.interactedWithNote` true (`self.BPPlayerRef`)))

(event `DropItem`
  (bind _returnvalue (`GameplayStatics.GetPlayerController` 0))
  ;[0 0 0] Drop Note and remove from the viewport
  (set `self.HasBeenPicked` false)
  (`Widget.RemoveFromParent` (`self.WB Note Ref`))
  (`self.SetActorHiddenInGame` false)
  (`Controller.SetIgnoreMoveInput` _returnvalue false)
  (`Controller.SetIgnoreLookInput` _returnvalue false))

(fn `UserConstructionScript`
  (`parent.UserConstructionScript`))