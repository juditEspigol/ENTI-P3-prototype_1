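; Red flickering spot light actor that can be switched on or off through the SetLight event.
; From BeginPlay, a Delay-driven loop sets the SpotLight to a random intensity within Min and Max, then waits a random time within TimeMin and TimeMax.
; SetLight stores the LightOfff flag and re-enters that logic, which either zeroes the intensity or resumes flickering.
; The loop ends after a delay once the flag is set.
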(event `self.ReceiveBeginPlay`
  (if (`self.LightOfff`) :!label _label
    (`LightComponent.SetIntensity` (`self.SpotLight`) 0.0)
    (else
      (`LightComponent.SetIntensity` (`self.SpotLight`) (`KismetMathLibrary.RandomFloatInRange` (`self.Min`) (`self.Max`)) :!label _label_2)
      (`KismetSystemLibrary.Delay` (`KismetMathLibrary.RandomFloatInRange` (`self.TimeMin`) (`self.TimeMax`)))
      (if (not (`self.LightOfff`))
        (goto _label_2)))))

(event `SetLight`
  (params (LihtsOff :type Boolean))
  (set `self.LightOfff` LihtsOff)
  (goto _label))

(fn `UserConstructionScript`)