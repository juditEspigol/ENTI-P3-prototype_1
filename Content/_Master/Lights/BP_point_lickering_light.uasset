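; Light Blueprint that makes its SpotLight flicker, despite the "point" in the asset name.
; From BeginPlay, a self-repeating Delay loop sets a random intensity between the Min and Max variables, then waits a random time between TimeMin and TimeMax.
; A hard-coded false branch leaves a one-shot random intensity path with fixed bounds unused.
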(event `self.ReceiveBeginPlay`
  (if false
    (`LightComponent.SetIntensity` (`self.SpotLight`) (`KismetMathLibrary.RandomFloatInRange` 5000.0 10000.0))
    (else
      (`LightComponent.SetIntensity` (`self.SpotLight`) (`KismetMathLibrary.RandomFloatInRange` (`self.Min`) (`self.Max`)) :!label _label)
      (`KismetSystemLibrary.Delay` (`KismetMathLibrary.RandomFloatInRange` (`self.TimeMin`) (`self.TimeMax`)))
      (goto _label))))

(fn `UserConstructionScript`)