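; Rect light actor that flickers randomly during play until it is switched off.
; On BeginPlay a delay loop sets the RectLight to a random intensity between Min and Max, then waits a random interval of up to half a second.
; The LightsOff event sets the Off flag, which ends the loop, and drops the intensity to zero; no event here restarts the flicker.
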(event `self.ReceiveBeginPlay`
  (if (not (`self.Off`))
    (`LightComponent.SetIntensity` (`self.RectLight`) (`KismetMathLibrary.RandomFloatInRange` (`self.Min`) (`self.Max`)) :!label _label)
    (`KismetSystemLibrary.Delay` (`KismetMathLibrary.RandomFloatInRange` 0.0 0.5))
    (if (not (`self.Off`))
      (goto _label))))

(event `LightsOff`
  (set `self.Off` true)
  (`LightComponent.SetIntensity` (`self.RectLight`) 0.0))

(fn `UserConstructionScript`)